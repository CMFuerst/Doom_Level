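; BP_Walking_Regina is a character that wanders the navmesh on its own at a randomized walking speed.
; BeginPlay picks a random speed and applies it to the movement component's max walk speed.
; Tick issues AI MoveTo toward a random navigable point within WalkRadius of its current location whenever it is not walking.
; A Walking flag blocks new requests until the move succeeds or fails, then the cycle repeats.
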(event `self.ReceiveBeginPlay`
  (bind _output_get (set `self.Walk_Speed` (`KismetMathLibrary.RandomFloatInRange` 100.0 450.0)))
  (set `CharacterMovementComponent.MaxWalkSpeed` _output_get (`self.CharacterMovement`)))

(event `self.ReceiveTick`
  (params (DeltaSeconds :type "Float (single-precision)"))
  (if (not (`self.Walking`))
    (`|AIMoveTo` self (`NavigationSystemV1.K2_GetRandomLocationInNavigableRadius` (`self.K2_GetActorLocation`) (`self.Walk_Radius`) null null) null
      (:`then`
        (set `self.Walking` true))
      (:`OnSuccess`
        (set `self.Walking` false :!label _label))
      (:`OnFail`
        (goto _label)))))

(fn `UserConstructionScript`)